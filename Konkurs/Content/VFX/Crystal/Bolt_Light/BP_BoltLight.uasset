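; BP_BoltLight is an interactive lightning bolt VFX actor that plays one of two effects when E is pressed.
; Box overlap enables input and briefly shows a PressE prompt; leaving disables input and hides it.
; A FlipFlop alternates two timelines, each animating E1's material parameter and a particle system's T1 vector.
; Timeline events activate the particles, play a flash sound and briefly reveal end effects, including smoke on the second.
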(event `self.Box.OnComponentBeginOverlap`
  (params (OverlappedComponent :type "PrimitiveComponent Object Reference") (OtherActor :type "Actor Object Reference") (OtherComp :type "PrimitiveComponent Object Reference") (OtherBodyIndex :type Integer) (bFromSweep :type Boolean) (SweepResult :type "HitResult Structure (by ref)"))
  (bind _press_e (`self.Press E`))
  (`self.EnableInput` (`GameplayStatics.GetPlayerController` 0))
  (`SceneComponent.SetVisibility` _press_e true false)
  (`KismetSystemLibrary.Delay` 5.0)
  (`SceneComponent.SetVisibility` _press_e false false))

(event `self.Box.OnComponentEndOverlap`
  (params (OverlappedComponent :type "PrimitiveComponent Object Reference") (OtherActor :type "Actor Object Reference") (OtherComp :type "PrimitiveComponent Object Reference") (OtherBodyIndex :type Integer))
  (`self.DisableInput` (`GameplayStatics.GetPlayerController` 0))
  (`SceneComponent.SetVisibility` (`self.Press E`) false false))

(event `Key|E`
  (params (Key :type "Key Structure"))
  (bind _smoke (`self.Smoke`))
  (bind _ps_light1 (`self.PS_light1`))
  (bind _ps_light (`self.PS_light`))
  (bind _e3 (`self.E3`))
  (:`Pressed`
    (`/Engine/EditorBlueprintResources/StandardMacros.FlipFlop`
      (:`A`
        (bind (_direction _e1 _bolt_trackx _bolt_tracky _bolt_trackz) (`Timeline|VFX` :!via `PlayFromStart`)
          (:`Update`
            (`MeshComponent.SetScalarParameterValueOnMaterials` (`self.E1`) "x" _e1)
            (`FXSystemComponent.SetVectorParameter` _ps_light "T1" (`KismetMathLibrary.MakeVector` _bolt_trackx _bolt_tracky _bolt_trackz)))
          (:`Bolt`
            (`ActorComponent.SetActive` _ps_light true false))
          (:`End`
            (`SceneComponent.SetVisibility` _e3 true false)
            (`SceneComponent.SetVisibility` (`self.E4`) true false)
            (`KismetSystemLibrary.Delay` 2.0)
            (`SceneComponent.SetVisibility` _e3 false false)
            (`SceneComponent.SetVisibility` (`self.E4`) false false))
          (:`Sound`
            (`GameplayStatics.PlaySound2D` "/Game/VFX/Crystal/Bolt_Light/FlashOne.FlashOne" 1.0 1.0 0.0 null null))))
      (:`B`
        (bind (_direction_2 _e1_2 _bolt_trackx_2 _bolt_tracky_2 _bolt_trackz_2) (`Timeline|Timeline` :!via `PlayFromStart`)
          (:`Update`
            (`MeshComponent.SetScalarParameterValueOnMaterials` (`self.E1`) "x" _e1_2)
            (`FXSystemComponent.SetVectorParameter` _ps_light1 "T1" (`KismetMathLibrary.MakeVector` (* 195.0 _bolt_trackx_2) (* -95.0 _bolt_tracky_2) (* 15.0 _bolt_trackz_2))))
          (:`Bolt`
            (`ActorComponent.SetActive` _ps_light1 true false))
          (:`End`
            (`SceneComponent.SetVisibility` _smoke true false)
            (`SceneComponent.SetVisibility` _smoke true false)
            (`KismetSystemLibrary.Delay` 0.5)
            (`SceneComponent.SetVisibility` _smoke false false)
            (`SceneComponent.SetVisibility` _smoke false false))
          (:`Sound`
            (`GameplayStatics.PlaySound2D` "/Game/VFX/Crystal/Bolt_Light/FlashOne.FlashOne" 1.0 1.0 0.0 null null)))))))

(fn `UserConstructionScript`)