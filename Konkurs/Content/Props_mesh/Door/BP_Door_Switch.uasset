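; Sliding door with three moving panels that the player toggles with an input action, usable only while the first-person character's SwitchON flag is set.
; A trigger box enables input on overlap and briefly shows either a press-E or need-energy prompt.
; A timeline slides the left, right and upper panels, playing forward or reversing based on DoorOpen, while DoorTrack blocks presses until it finishes.
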(event `self.Box_colisoin.OnComponentBeginOverlap`
  (params (OverlappedComponent :type "PrimitiveComponent Object Reference") (OtherActor :type "Actor Object Reference") (OtherComp :type "PrimitiveComponent Object Reference") (OtherBodyIndex :type Integer) (bFromSweep :type Boolean) (SweepResult :type "HitResult Structure (by ref)"))
  (bind _press_e (`self.Press E`))
  (bind _need_energy (`self.Need Energy`))
  (`self.EnableInput` (`GameplayStatics.GetPlayerController` 0))
  (bind _asbp_first_person_character (cast `/Game/FirstPerson/Blueprints/BP_FirstPersonCharacter` (`GameplayStatics.GetPlayerCharacter` 0)))
  (if (`/Game/FirstPerson/Blueprints/BP_FirstPersonCharacter.SwitchON` _asbp_first_person_character)
    (`SceneComponent.SetVisibility` _press_e true false)
    (`KismetSystemLibrary.Delay` 1.5)
    (`SceneComponent.SetVisibility` _press_e false false)
    (else
      (`SceneComponent.SetVisibility` _need_energy true false)
      (`KismetSystemLibrary.Delay` 1.5)
      (`SceneComponent.SetVisibility` _need_energy false false))))

(event `self.Box_colisoin.OnComponentEndOverlap`
  (params (OverlappedComponent :type "PrimitiveComponent Object Reference") (OtherActor :type "Actor Object Reference") (OtherComp :type "PrimitiveComponent Object Reference") (OtherBodyIndex :type Integer))
  (`self.DisableInput` (`GameplayStatics.GetPlayerController` 0))
  (`SceneComponent.SetVisibility` (`self.Press E`) false false)
  (`SceneComponent.SetVisibility` (`self.Need Energy`) false false))

(event `InputAction|Switch_Door_light`
  (params (Key :type "Key Structure"))
  (:`Pressed`
    (bind _asbp_first_person_character (cast `/Game/FirstPerson/Blueprints/BP_FirstPersonCharacter` (`GameplayStatics.GetPlayerCharacter` 0)))
    (if (`/Game/FirstPerson/Blueprints/BP_FirstPersonCharacter.SwitchON` _asbp_first_person_character)
      (if (`self.DoorTrack`)
        (if (`self.DoorOpen`)
          (set `self.DoorTrack` false)
          (set `self.Close_Door` (not (`self.Close_Door`)))
          (if true
            (bind (_direction _newtrack_0 _newtrack_1) (`Timeline|Timeline` :!label _label)
              (:`Update`
                (`SceneComponent.K2_SetRelativeLocation` (`self.Door_Up`) (`KismetMathLibrary.MakeVector` 0.0 0.0 (* 40.0 _newtrack_1)) false false)
                (set `self.Close_Door` (> _newtrack_0 39.0))
                (`SceneComponent.K2_SetRelativeLocation` (`self.Door_Left`) (`KismetMathLibrary.MakeVector` 0.0 (* _newtrack_0 -40.0)) false false)
                (`SceneComponent.K2_SetRelativeLocation` (`self.Door_Right`) (`KismetMathLibrary.MakeVector` 0.0 (* _newtrack_0 40.0)) false false)
                (set `self.DoorOpen` (not (> _newtrack_0 0.0)))
                (set `self.DoorOpen` (not (> _newtrack_1 0.0))))
              (:`Finished`
                (set `self.DoorTrack` true)))
            (else
              (goto _label :!via `ReverseFromEnd`)))
          (else
            (set `self.DoorTrack` false)
            (goto _label :!via `ReverseFromEnd`)))))))

(fn `UserConstructionScript`)