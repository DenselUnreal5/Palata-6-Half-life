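; Sci-fi sliding door that opens when anything overlaps its Box trigger and closes when an overlap ends.
; One timeline drives three panels through relative location: DoorUp rises while DoorLeft and DoorRight slide apart along Y.
; Opening plays a 2D sound; closing is silent and reverses the timeline from its end, even if opening is unfinished.
; Delay-based sound and reopen chains are left unwired and never run.
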(event `self.Box.OnComponentBeginOverlap`
  (params (OverlappedComponent :type "PrimitiveComponent Object Reference") (OtherActor :type "Actor Object Reference") (OtherComp :type "PrimitiveComponent Object Reference") (OtherBodyIndex :type Integer) (bFromSweep :type Boolean) (SweepResult :type "HitResult Structure (by ref)"))
  (`GameplayStatics.SpawnSound2D` "/Game/Props_mesh/Door/Sound/Sound-Effects-Sci-Fi-Door-Opening-or-Closing.Sound-Effects-Sci-Fi-Door-Opening-or-Closing" 1.0 1.0 0.0 null)
  (bind (_direction _newtrack_0 _newtrack_1) (`Timeline|Timeline_1` :!label _label)
    (:`Update`
      (`SceneComponent.K2_SetRelativeLocation` (`self.Door_Up`) (`KismetMathLibrary.MakeVector` 0.0 0.0 (* 40.0 _newtrack_1)) false false)
      (`SceneComponent.K2_SetRelativeLocation` (`self.Door_Left`) (`KismetMathLibrary.MakeVector` 0.0 (* _newtrack_0 40.0)) false false)
      (`SceneComponent.K2_SetRelativeLocation` (`self.Door_Right`) (`KismetMathLibrary.MakeVector` 0.0 (* _newtrack_0 -40.0)) false false))))

(event `self.Box.OnComponentEndOverlap`
  (params (OverlappedComponent :type "PrimitiveComponent Object Reference") (OtherActor :type "Actor Object Reference") (OtherComp :type "PrimitiveComponent Object Reference") (OtherBodyIndex :type Integer))
  (goto _label :!via `ReverseFromEnd`))

(fn `UserConstructionScript`)