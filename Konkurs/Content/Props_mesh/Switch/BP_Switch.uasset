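; Interactable lever switch prop that sets the SwitchON flag on the first-person player character.
; Overlapping its collision enables input on the switch and shows a PressE prompt for two seconds; leaving disables input and hides the prompt.
; The Switch_Door_Light action sets the flag, plays a 2D lever sound and runs a timeline that slides the switch component along X and Z.
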(event `self.Colision.OnComponentBeginOverlap`
  (params (OverlappedComponent :type "PrimitiveComponent Object Reference") (OtherActor :type "Actor Object Reference") (OtherComp :type "PrimitiveComponent Object Reference") (OtherBodyIndex :type Integer) (bFromSweep :type Boolean) (SweepResult :type "HitResult Structure (by ref)"))
  (bind _press_e (`self.Press E`))
  (`self.EnableInput` (`GameplayStatics.GetPlayerController` 0))
  (`SceneComponent.SetVisibility` _press_e true false)
  (`KismetSystemLibrary.Delay` 2.0)
  (`SceneComponent.SetVisibility` _press_e false false :!label _label))

(event `self.Colision.OnComponentEndOverlap`
  (params (OverlappedComponent :type "PrimitiveComponent Object Reference") (OtherActor :type "Actor Object Reference") (OtherComp :type "PrimitiveComponent Object Reference") (OtherBodyIndex :type Integer))
  (`self.DisableInput` (`GameplayStatics.GetPlayerController` 0))
  (`SceneComponent.SetVisibility` (`self.Press E`) false false)
  (goto _label))

(event `InputAction|Switch_Door_Light`
  (params (Key :type "Key Structure"))
  (:`Pressed`
    (bind _asbp_first_person_character (cast `/Game/FirstPerson/Blueprints/BP_FirstPersonCharacter` (`GameplayStatics.GetPlayerCharacter` 0)))
    (set `/Game/FirstPerson/Blueprints/BP_FirstPersonCharacter.SwitchON` true _asbp_first_person_character)
    (`GameplayStatics.SpawnSound2D` "/Game/Props_mesh/Switch/Sound/lever1.lever1" 1.0 1.0 0.0 null)
    (bind (_direction _time_switch _for_z) (`Timeline|Switch_Time`)
      (:`Update`
        (`SceneComponent.K2_SetRelativeLocation` (`self.Switch`) (`KismetMathLibrary.MakeVector` (* _time_switch 5.0) 0.0 (* _for_z -18.0)) false false)))))

(fn `UserConstructionScript`)