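; BP_Flash is a one-shot trigger actor that stages a double lightning strike when something overlaps its box.
; The overlap calls the flash event, which plays a 2D sound and destroys the box so it cannot retrigger.
; Timed delays briefly show and hide the FlashLight component, then repeat the sound and flash for a second strike.
; The overlapping actor is not filtered.
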(event `self.Box.OnComponentBeginOverlap`
  (params (OverlappedComponent :type "PrimitiveComponent Object Reference") (OtherActor :type "Actor Object Reference") (OtherComp :type "PrimitiveComponent Object Reference") (OtherBodyIndex :type Integer) (bFromSweep :type Boolean) (SweepResult :type "HitResult Structure (by ref)"))
  ;[1 1 1] запуск эвента"Молния"
  (`self.Flash_Event`))

(event `Flash_Event`
  (bind _flashlight (`self.flashLight`))
  (bind _flashlight_2 (`self.flashLight`))
  ;[1 1 1] удар молнии
  (`GameplayStatics.PlaySound2D` "/Game/Sound/Effect/FlashOne/FlashOne.FlashOne" 1.0 1.0 0.0 null null)
  (`ActorComponent.K2_DestroyComponent` (`self.Box`))
  (`SceneComponent.SetVisibility` _flashlight_2 true false)
  (`KismetSystemLibrary.Delay` 0.2)
  (`SceneComponent.SetVisibility` _flashlight_2 false false)
  (`KismetSystemLibrary.Delay` 1.0)
  ;;[1 1 1] второй удар молнии
  (`GameplayStatics.PlaySound2D` "/Game/Sound/Effect/FlashOne/FlashOne.FlashOne" 1.0 1.0 0.0 null null)
  (`SceneComponent.SetVisibility` _flashlight true false)
  (`KismetSystemLibrary.Delay` 0.2)
  (`SceneComponent.SetVisibility` _flashlight false false))

(fn `UserConstructionScript`)