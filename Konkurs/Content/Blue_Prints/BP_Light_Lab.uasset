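; BP_Light_Lab is a spotlight Blueprint whose visibility depends on the player's switch state.
; On BeginPlay it hides its SpotLight, casts the player character to BP_FirstPersonCharacter and reads SwitchON.
; If that is true, the light turns on after a short delay; otherwise it stays hidden.
; The switch is checked only once at BeginPlay, so later changes to it do not affect the light.
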(event `self.ReceiveBeginPlay`
  (`SceneComponent.SetVisibility` (`self.SpotLight`) false false)
  (bind _asbp_first_person_character (cast `/Game/FirstPerson/Blueprints/BP_FirstPersonCharacter` (`GameplayStatics.GetPlayerCharacter` 0)))
  (if (`/Game/FirstPerson/Blueprints/BP_FirstPersonCharacter.SwitchON` _asbp_first_person_character)
    (`KismetSystemLibrary.Delay` 2.0)
    (`SceneComponent.SetVisibility` (`self.SpotLight`) true false)
    (else
      (`SceneComponent.SetVisibility` (`self.SpotLight`) false false))))

(fn `UserConstructionScript`)