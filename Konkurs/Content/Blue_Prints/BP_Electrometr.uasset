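; BP_Electrometr is an interactable electrometer prop that shows a "press E" hint and plays a sound when used.
; Entering its box trigger enables player input on the actor and shows the hint for three seconds, while leaving disables input and hides it.
; Pressing E checks that the player is the first-person character, then plays the Not_active 2D sound.
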(event `self.Box.OnComponentBeginOverlap`
  (params (OverlappedComponent :type "PrimitiveComponent Object Reference") (OtherActor :type "Actor Object Reference") (OtherComp :type "PrimitiveComponent Object Reference") (OtherBodyIndex :type Integer) (bFromSweep :type Boolean) (SweepResult :type "HitResult Structure (by ref)"))
  (bind _press_e (`self.Press E`))
  ;[1 1 1] подсказка
  (`self.EnableInput` (`GameplayStatics.GetPlayerController` 0))
  (`SceneComponent.SetVisibility` _press_e true false)
  (`KismetSystemLibrary.Delay` 3.0)
  (`SceneComponent.SetVisibility` _press_e false false))

(event `self.Box.OnComponentEndOverlap`
  (params (OverlappedComponent :type "PrimitiveComponent Object Reference") (OtherActor :type "Actor Object Reference") (OtherComp :type "PrimitiveComponent Object Reference") (OtherBodyIndex :type Integer))
  ;[1 1 1] подсказка
  (`self.DisableInput` (`GameplayStatics.GetPlayerController` 0))
  (`SceneComponent.SetVisibility` (`self.Press E`) false false))

(event `Key|E`
  (params (Key :type "Key Structure"))
  ;[1 1 1] звуковой эффект
  (:`Pressed`
    (cast `/Game/FirstPerson/Blueprints/BP_FirstPersonCharacter` (`GameplayStatics.GetPlayerCharacter` 0))
    (`GameplayStatics.PlaySound2D` "/Game/Sound/Button_sound/not_active.not_active" 1.0 1.0 0.0 null null)))

(fn `UserConstructionScript`)