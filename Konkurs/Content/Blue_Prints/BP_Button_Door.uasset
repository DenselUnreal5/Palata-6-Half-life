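; BP_Button_Door is a two-button switch (green and red) that animates with sound when the player presses Switch_Door_light nearby; no door logic is present.
; A box overlap toggles input, and presses require the first-person character's SwitchON flag.
; Nested FlipFlops alternate between buttons, each playing or reversing its Timeline to slide along X.
; Dynamic-material logic for emissive switching is disconnected and never runs.
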(event `self.Box.OnComponentBeginOverlap`
  (params (OverlappedComponent :type "PrimitiveComponent Object Reference") (OtherActor :type "Actor Object Reference") (OtherComp :type "PrimitiveComponent Object Reference") (OtherBodyIndex :type Integer) (bFromSweep :type Boolean) (SweepResult :type "HitResult Structure (by ref)"))
  ;[1 1 1] Зашел/Вышел вкл/выкл эвентов
  (`self.EnableInput` (`GameplayStatics.GetPlayerController` 0)))

(event `self.Box.OnComponentEndOverlap`
  (params (OverlappedComponent :type "PrimitiveComponent Object Reference") (OtherActor :type "Actor Object Reference") (OtherComp :type "PrimitiveComponent Object Reference") (OtherBodyIndex :type Integer))
  ;[1 1 1] Зашел/Вышел вкл/выкл эвентов
  (`self.DisableInput` (`GameplayStatics.GetPlayerController` 0)))

(event `InputAction|Switch_Door_light`
  (params (Key :type "Key Structure"))
  ;[1 1 1] вкл/выкл анимации
  (:`Pressed`
    (bind _asbp_first_person_character (cast `/Game/FirstPerson/Blueprints/BP_FirstPersonCharacter` (`GameplayStatics.GetPlayerCharacter` 0)))
    (if (`/Game/FirstPerson/Blueprints/BP_FirstPersonCharacter.SwitchON` _asbp_first_person_character)
      (`GameplayStatics.PlaySound2D` "/Game/Sound/Button_sound/Button_sound.Button_sound" 1.0 1.0 0.0 null null)
      (`/Engine/EditorBlueprintResources/StandardMacros.FlipFlop`
        (:`A`
          (`/Engine/EditorBlueprintResources/StandardMacros.FlipFlop`
            (:`A`
              (bind (_direction _newtrack_0) (`Timeline|Timeline` :!label _label)
                (:`Update`
                  (`SceneComponent.K2_SetRelativeLocation` (`self.ButtonGreen`) (`KismetMathLibrary.MakeVector` (* _newtrack_0 -1.0)) false false))))
            (:`B`
              (goto _label :!via `Reverse`))))
        (:`B`
          (`/Engine/EditorBlueprintResources/StandardMacros.FlipFlop`
            (:`A`
              (bind (_direction_2 _newtrack_0_2) (`Timeline|Timeline_0` :!label _label_2)
                (:`Update`
                  (`SceneComponent.K2_SetRelativeLocation` (`self.ButtonRed`) (`KismetMathLibrary.MakeVector` (* _newtrack_0_2 -1.0)) false false))))
            (:`B`
              (goto _label_2 :!via `Reverse`))))))))

(fn `UserConstructionScript`)