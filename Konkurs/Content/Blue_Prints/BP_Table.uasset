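; BP_Table is an interactive table with a sliding shelf that the player opens and closes with a key press.
; Box overlap enables input and briefly shows the PressE prompt; leaving disables input and hides it.
; On Switch_Door_light, if the character's SwitchON is true, a FlipFlop alternately plays and reverses the ShelfAnim timeline, which drives the shelf's relative Z location.
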(event `self.Box.OnComponentBeginOverlap`
  (params (OverlappedComponent :type "PrimitiveComponent Object Reference") (OtherActor :type "Actor Object Reference") (OtherComp :type "PrimitiveComponent Object Reference") (OtherBodyIndex :type Integer) (bFromSweep :type Boolean) (SweepResult :type "HitResult Structure (by ref)"))
  (bind _press_e (`self.Press E`))
  ;[1 1 1] Отображение нажми на Е
  (`self.EnableInput` (`GameplayStatics.GetPlayerController` 0))
  (cast `/Game/FirstPerson/Blueprints/BP_FirstPersonCharacter` (`GameplayStatics.GetPlayerCharacter` 0))
  (`SceneComponent.SetVisibility` _press_e true false)
  (`KismetSystemLibrary.Delay` 2.0)
  (`SceneComponent.SetVisibility` _press_e false false))

(event `self.Box.OnComponentEndOverlap`
  (params (OverlappedComponent :type "PrimitiveComponent Object Reference") (OtherActor :type "Actor Object Reference") (OtherComp :type "PrimitiveComponent Object Reference") (OtherBodyIndex :type Integer))
  ;[1 1 1] Отображение нажми на Е
  (`self.DisableInput` (`GameplayStatics.GetPlayerController` 0))
  (`SceneComponent.SetVisibility` (`self.Press E`) false false))

(event `InputAction|Switch_Door_light`
  (params (Key :type "Key Structure"))
  ;[1 1 1] после нажатия Е идет анимация выдвижного шкафа
  (:`Pressed`
    (bind _asbp_first_person_character (cast `/Game/FirstPerson/Blueprints/BP_FirstPersonCharacter` (`GameplayStatics.GetPlayerCharacter` 0)))
    (if (`/Game/FirstPerson/Blueprints/BP_FirstPersonCharacter.SwitchON` _asbp_first_person_character)
      (`/Engine/EditorBlueprintResources/StandardMacros.FlipFlop`
        (:`A`
          (bind (_direction _move) (`Timeline|Shelf Anim` :!label _label)
            (:`Update`
              (`SceneComponent.K2_SetRelativeLocation` (`self.shelf`) (`KismetMathLibrary.MakeVector` 0.0 0.0 (* _move -85.0)) false false))))
        (:`B`
          (goto _label :!via `Reverse`))))))

(fn `UserConstructionScript`)