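; BP_Door is an automatic three-panel door that opens when something enters its Box trigger and closes when it leaves.
; Overlap events play or reverse one timeline, whose two tracks slide DoorUp along Z and DoorLeft and DoorRight apart along Y.
; Each event also spawns a 2D open or close sound, which a comment notes can stack when passing through quickly.
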(event `self.Box.OnComponentBeginOverlap`
  (params (OverlappedComponent :type "PrimitiveComponent Object Reference") (OtherActor :type "Actor Object Reference") (OtherComp :type "PrimitiveComponent Object Reference") (OtherBodyIndex :type Integer) (bFromSweep :type Boolean) (SweepResult :type "HitResult Structure (by ref)"))
  ;[1 1 1] Автоматические двери открыть/закрыть, не смог решить проблему со звуком до конца, если очень быстро проходить через BOX звук накладывается друг на друга
  (`GameplayStatics.SpawnSound2D` "/Game/Sound/Door_sound/Open_door.Open_door" 1.0 1.0 0.0 null)
  (bind (_direction _newtrack_0 _newtrack_1) (`Timeline|Timeline_1` :!label _label)
    (:`Update`
      (`SceneComponent.K2_SetRelativeLocation` (`self.Door_Up`) (`KismetMathLibrary.MakeVector` 0.0 0.0 (* 40.0 _newtrack_1)) false false)
      (`SceneComponent.K2_SetRelativeLocation` (`self.Door_Left`) (`KismetMathLibrary.MakeVector` 0.0 (* _newtrack_0 40.0)) false false)
      (`SceneComponent.K2_SetRelativeLocation` (`self.Door_Right`) (`KismetMathLibrary.MakeVector` 0.0 (* _newtrack_0 -40.0)) false false))))

(event `self.Box.OnComponentEndOverlap`
  (params (OverlappedComponent :type "PrimitiveComponent Object Reference") (OtherActor :type "Actor Object Reference") (OtherComp :type "PrimitiveComponent Object Reference") (OtherBodyIndex :type Integer))
  ;[1 1 1] Автоматические двери открыть/закрыть, не смог решить проблему со звуком до конца, если очень быстро проходить через BOX звук накладывается друг на друга
  (`GameplayStatics.SpawnSound2D` "/Game/Sound/Door_sound/Close_Door.Close_Door" 1.0 1.0 0.0 null)
  (goto _label :!via `Reverse`))

(fn `UserConstructionScript`)