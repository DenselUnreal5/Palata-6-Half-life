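; BP_Door_Switch is a sliding door that the first-person player opens and closes with E.
; Its collision box enables input on overlap, briefly shows "Press E" prompts and swaps door and button materials and light colors to greenish, reverting to red on exit.
; E drives a FlipFlop that plays or reverses a Timeline moving the left, right and upper panels, with sound.
; Despite the comment, no power-switch check appears.
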(event `self.ReceiveBeginPlay`)

(event `self.Box_colisoin.OnComponentBeginOverlap`
  (params (OverlappedComponent :type "PrimitiveComponent Object Reference") (OtherActor :type "Actor Object Reference") (OtherComp :type "PrimitiveComponent Object Reference") (OtherBodyIndex :type Integer) (bFromSweep :type Boolean) (SweepResult :type "HitResult Structure (by ref)"))
  (bind _linearcolor (make `LinearColor` 0.7 1.0 0.5))
  (bind _press_e (`self.Press E`))
  ;[1 1 1] Надписи
  (`self.EnableInput` (`GameplayStatics.GetPlayerController` 0))
  (cast `/Game/FirstPerson/Blueprints/BP_FirstPersonCharacter` (`GameplayStatics.GetPlayerCharacter` 0))
  (`PrimitiveComponent.CreateDynamicMaterialInstance` (`self.Door_Right`) 0 "/Game/Materials/Materials_props_inst/MI_props_emissev_Inst.MI_props_emissev_Inst" "None")
  (`PrimitiveComponent.CreateDynamicMaterialInstance` (`self.Door_Left`) 0 "/Game/Materials/Materials_props_inst/MI_props_emissev_Inst.MI_props_emissev_Inst" "None")
  (`PrimitiveComponent.CreateDynamicMaterialInstance` (`self.DoorFrame`) 0 "/Game/Materials/Materials_props_inst/MI_props_emissev_Inst.MI_props_emissev_Inst" "None")
  (`PrimitiveComponent.CreateDynamicMaterialInstance` (`self.ButtonGreen`) 0 "/Game/Materials/Materials_props_inst/Range_hood2.Range_hood2" "None")
  (`PrimitiveComponent.CreateDynamicMaterialInstance` (`self.ButtonRed`) 0 "/Game/Materials/Materials_props_inst/Range_hood2.Range_hood2" "None")
  (`PrimitiveComponent.CreateDynamicMaterialInstance` (`self.ButtonGreen1`) 0 "/Game/Materials/Materials_props_inst/Range_hood2.Range_hood2" "None")
  (`PrimitiveComponent.CreateDynamicMaterialInstance` (`self.ButtonRed1`) 0 "/Game/Materials/Materials_props_inst/Range_hood2.Range_hood2" "None")
  (`LightComponent.SetLightColor` (`self.PointLight`) _linearcolor true)
  (`LightComponent.SetLightColor` (`self.PointLight1`) _linearcolor true)
  (`SceneComponent.SetVisibility` _press_e true false)
  (`SceneComponent.SetVisibility` (`self.Press E1`) true false)
  (`KismetSystemLibrary.Delay` 2.0)
  (`SceneComponent.SetVisibility` _press_e false false)
  (`SceneComponent.SetVisibility` (`self.Press E1`) false false))

(event `self.Box_colisoin.OnComponentEndOverlap`
  (params (OverlappedComponent :type "PrimitiveComponent Object Reference") (OtherActor :type "Actor Object Reference") (OtherComp :type "PrimitiveComponent Object Reference") (OtherBodyIndex :type Integer))
  (bind _linearcolor (make `LinearColor` 1.0 0.04 0.1))
  ;[1 1 1] Надписи
  (`self.DisableInput` (`GameplayStatics.GetPlayerController` 0))
  (`SceneComponent.SetVisibility` (`self.Press E`) false false)
  (`PrimitiveComponent.CreateDynamicMaterialInstance` (`self.Door_Right`) 0 "/Game/Materials/Materials_props_inst/Door_Onst.Door_Onst" "None")
  (`PrimitiveComponent.CreateDynamicMaterialInstance` (`self.Door_Left`) 0 "/Game/Materials/Materials_props_inst/Door_Onst.Door_Onst" "None")
  (`PrimitiveComponent.CreateDynamicMaterialInstance` (`self.DoorFrame`) 0 "/Game/Materials/Materials_props_inst/Door_Onst.Door_Onst" "None")
  (`PrimitiveComponent.CreateDynamicMaterialInstance` (`self.ButtonGreen`) 0 "/Game/Materials/Materials_props_inst/Range_hood_NOTEmmisive.Range_hood_NOTEmmisive" "None")
  (`PrimitiveComponent.CreateDynamicMaterialInstance` (`self.ButtonRed`) 0 "/Game/Materials/Materials_props_inst/Range_hood_NOTEmmisive.Range_hood_NOTEmmisive" "None")
  (`PrimitiveComponent.CreateDynamicMaterialInstance` (`self.ButtonGreen1`) 0 "/Game/Materials/Materials_props_inst/Range_hood_NOTEmmisive.Range_hood_NOTEmmisive" "None")
  (`PrimitiveComponent.CreateDynamicMaterialInstance` (`self.ButtonRed1`) 0 "/Game/Materials/Materials_props_inst/Range_hood_NOTEmmisive.Range_hood_NOTEmmisive" "None")
  (`LightComponent.SetLightColor` (`self.PointLight`) _linearcolor true)
  (`LightComponent.SetLightColor` (`self.PointLight1`) _linearcolor true))

(event `Key|E`
  (params (Key :type "Key Structure"))
  ;[1 1 1] Открытие и закрытие двери при определенных условиях (рубильник должен быть включен) проблема дверь закрывается не сразу, не могу найти причину
  (:`Pressed`
    (cast `/Game/FirstPerson/Blueprints/BP_FirstPersonCharacter` (`GameplayStatics.GetPlayerCharacter` 0))
    (`/Engine/EditorBlueprintResources/StandardMacros.FlipFlop`
      (:`A`
        (`GameplayStatics.SpawnSound2D` "/Game/Sound/Door_sound/Open_door.Open_door" 1.0 1.0 0.0 null)
        (bind (_direction _newtrack_0 _newtrack_1) (`Timeline|Timeline` :!label _label)
          (:`Update`
            (`SceneComponent.K2_SetRelativeLocation` (`self.Door_Up`) (`KismetMathLibrary.MakeVector` 0.0 0.0 (* 40.0 _newtrack_1)) false false)
            (`SceneComponent.K2_SetRelativeLocation` (`self.Door_Left`) (`KismetMathLibrary.MakeVector` 0.0 (* _newtrack_0 -40.0)) false false)
            (`SceneComponent.K2_SetRelativeLocation` (`self.Door_Right`) (`KismetMathLibrary.MakeVector` 0.0 (* _newtrack_0 40.0)) false false))))
      (:`B`
        (`GameplayStatics.SpawnSound2D` "/Game/Sound/Door_sound/Open_door.Open_door" 1.0 1.0 0.0 null)
        (goto _label :!via `Reverse`)))))

(fn `UserConstructionScript`)