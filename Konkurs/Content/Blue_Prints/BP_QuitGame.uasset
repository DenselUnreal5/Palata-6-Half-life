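; BP_QuitGame is a trigger actor that lets the player leave to the main menu.
; Entering its Box enables input on the actor and shows the QuitGame hint for three seconds, while leaving disables input and hides it.
; Pressing E while input is enabled opens MainMenu_map, provided the player character is BP_FirstPersonCharacter.
; The overlap events do not check which actor enters or leaves.
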(event `self.Box.OnComponentBeginOverlap`
  (params (OverlappedComponent :type "PrimitiveComponent Object Reference") (OtherActor :type "Actor Object Reference") (OtherComp :type "PrimitiveComponent Object Reference") (OtherBodyIndex :type Integer) (bFromSweep :type Boolean) (SweepResult :type "HitResult Structure (by ref)"))
  (bind _quitgame (`self.QuitGame`))
  ;[1 1 1] подсказка
  (`self.EnableInput` (`GameplayStatics.GetPlayerController` 0))
  (`SceneComponent.SetVisibility` _quitgame true false)
  (`KismetSystemLibrary.Delay` 3.0)
  (`SceneComponent.SetVisibility` _quitgame false false))

(event `self.Box.OnComponentEndOverlap`
  (params (OverlappedComponent :type "PrimitiveComponent Object Reference") (OtherActor :type "Actor Object Reference") (OtherComp :type "PrimitiveComponent Object Reference") (OtherBodyIndex :type Integer))
  ;[1 1 1] подсказка
  (`self.DisableInput` (`GameplayStatics.GetPlayerController` 0))
  (`SceneComponent.SetVisibility` (`self.QuitGame`) false false))

(event `Key|E`
  (params (Key :type "Key Structure"))
  ;[1 1 1] Выйти из игры
  (:`Pressed`
    (cast `/Game/FirstPerson/Blueprints/BP_FirstPersonCharacter` (`GameplayStatics.GetPlayerCharacter` 0))
    (`GameplayStatics.OpenLevel` "MainMenu_map")))

(fn `UserConstructionScript`)