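; BP_Switch is an interactable lever that the player pulls with E while inside its collision volume.
; Overlap enables input and briefly shows the PressE prompt, while leaving disables input and hides it.
; Pressing E plays a lever sound and runs the Switch_Time timeline to pitch the Switch component downward.
; A FlipFlop alternates Play and PlayFromStart, so the lever never animates in reverse, and nothing else is triggered.
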(event `self.Colision.OnComponentBeginOverlap`
  (params (OverlappedComponent :type "PrimitiveComponent Object Reference") (OtherActor :type "Actor Object Reference") (OtherComp :type "PrimitiveComponent Object Reference") (OtherBodyIndex :type Integer) (bFromSweep :type Boolean) (SweepResult :type "HitResult Structure (by ref)"))
  (bind _press_e (`self.Press E`))
  ;[1 1 1] Активация надписей
  (`self.EnableInput` (`GameplayStatics.GetPlayerController` 0))
  (`SceneComponent.SetVisibility` _press_e true false)
  (`KismetSystemLibrary.Delay` 2.0)
  (`SceneComponent.SetVisibility` _press_e false false :!label _label))

(event `self.Colision.OnComponentEndOverlap`
  (params (OverlappedComponent :type "PrimitiveComponent Object Reference") (OtherActor :type "Actor Object Reference") (OtherComp :type "PrimitiveComponent Object Reference") (OtherBodyIndex :type Integer))
  ;[1 1 1] Активация надписей
  (`self.DisableInput` (`GameplayStatics.GetPlayerController` 0))
  (`SceneComponent.SetVisibility` (`self.Press E`) false false)
  (goto _label))

(event `Key|E`
  (params (Key :type "Key Structure"))
  ;[1 1 1] рычаг опускается
  (:`Pressed`
    (cast `/Game/FirstPerson/Blueprints/BP_FirstPersonCharacter` (`GameplayStatics.GetPlayerCharacter` 0))
    (`GameplayStatics.SpawnSound2D` "/Game/Sound/Switch_sound/lever1.lever1" 1.0 1.0 0.0 null)
    (`/Engine/EditorBlueprintResources/StandardMacros.FlipFlop`
      (:`A`
        (bind (_direction _time_switch _for_z _rotation) (`Timeline|Switch_Time` :!label _label_2)
          (:`Update`
            (`SceneComponent.K2_SetRelativeRotation` (`self.Switch`) (`KismetMathLibrary.MakeRotator` 0.0 (* _rotation -90.0)) false false))))
      (:`B`
        (goto _label_2 :!via `PlayFromStart`)))))

(fn `UserConstructionScript`)