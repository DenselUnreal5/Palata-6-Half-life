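; BP_Button is a two-button wall switch that toggles referenced spotlights when the player character's SwitchON flag is set.
; Overlapping Box enables input and briefly shows a PressE prompt.
; Switch_Door_light toggles the lights and uses nested FlipFlops to alternate green and red button timelines, or plays a failure sound without SwitchON.
; Tracker overlaps swap both buttons between emissive and non-emissive materials based on that flag.
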(event `self.Box.OnComponentBeginOverlap`
  (params (OverlappedComponent :type "PrimitiveComponent Object Reference") (OtherActor :type "Actor Object Reference") (OtherComp :type "PrimitiveComponent Object Reference") (OtherBodyIndex :type Integer) (bFromSweep :type Boolean) (SweepResult :type "HitResult Structure (by ref)"))
  (bind _press_e (`self.Press E`))
  ;[1 1 1] Навигация
  (`self.EnableInput` (`GameplayStatics.GetPlayerController` 0))
  (`SceneComponent.SetVisibility` _press_e true false)
  (`KismetSystemLibrary.Delay` 2.0)
  (`SceneComponent.SetVisibility` _press_e false false))

(event `self.Box.OnComponentEndOverlap`
  (params (OverlappedComponent :type "PrimitiveComponent Object Reference") (OtherActor :type "Actor Object Reference") (OtherComp :type "PrimitiveComponent Object Reference") (OtherBodyIndex :type Integer))
  ;[1 1 1] Навигация
  (`self.DisableInput` (`GameplayStatics.GetPlayerController` 0))
  (`SceneComponent.SetVisibility` (`self.Press E`) false false))

(event `InputAction|Switch_Door_light`
  (params (Key :type "Key Structure"))
  ;[1 1 1] вкл/выкл анимации
  (:`Pressed`
    (bind _asbp_first_person_character (cast `/Game/FirstPerson/Blueprints/BP_FirstPersonCharacter` (`GameplayStatics.GetPlayerCharacter` 0)))
    (if (`/Game/FirstPerson/Blueprints/BP_FirstPersonCharacter.SwitchON` _asbp_first_person_character)
      (`GameplayStatics.PlaySound2D` "/Game/Sound/Button_sound/Button_sound.Button_sound" 1.0 1.0 0.0 null null)
      (`/Engine/EditorBlueprintResources/StandardMacros.FlipFlop`
        (:`A`
          (`/Engine/EditorBlueprintResources/StandardMacros.FlipFlop`
            (:`A`
              (bind (_direction _newtrack_0) (`Timeline|Timeline` :!label _label)
                (:`Update`
                  (`SceneComponent.K2_SetRelativeLocation` (`self.ButtonGreen`) (`KismetMathLibrary.MakeVector` (* _newtrack_0 -1.0)) false false))))
            (:`B`
              (goto _label :!via `Reverse`))))
        (:`B`
          (`/Engine/EditorBlueprintResources/StandardMacros.FlipFlop`
            (:`A`
              (bind (_direction_2 _newtrack_0_2) (`Timeline|Timeline_0` :!label _label_2)
                (:`Update`
                  (`SceneComponent.K2_SetRelativeLocation` (`self.ButtonRed`) (`KismetMathLibrary.MakeVector` (* _newtrack_0_2 -1.0)) false false))))
            (:`B`
              (goto _label_2 :!via `Reverse`)))))
      (else
        (`GameplayStatics.SpawnSound2D` "/Game/Sound/Door_sound/DoorNotWork.DoorNotWork" 1.0 1.0 0.0 null)))))

(event `self.Tracker.OnComponentBeginOverlap`
  (params (OverlappedComponent :type "PrimitiveComponent Object Reference") (OtherActor :type "Actor Object Reference") (OtherComp :type "PrimitiveComponent Object Reference") (OtherBodyIndex :type Integer) (bFromSweep :type Boolean) (SweepResult :type "HitResult Structure (by ref)"))
  (bind _buttongreen (`self.ButtonGreen`))
  (bind _buttonred (`self.ButtonRed`))
  ;[1 1 1] Добавление емисии
  (bind _asbp_first_person_character (cast `/Game/FirstPerson/Blueprints/BP_FirstPersonCharacter` (`GameplayStatics.GetPlayerCharacter` 0) :!label _label_3))
  (if (`/Game/FirstPerson/Blueprints/BP_FirstPersonCharacter.SwitchON` _asbp_first_person_character)
    (`PrimitiveComponent.CreateDynamicMaterialInstance` _buttongreen 0 "/Game/Materials/Materials_props/Range_hood.Range_hood" "None")
    (`PrimitiveComponent.CreateDynamicMaterialInstance` _buttonred 0 "/Game/Materials/Materials_props/Range_hood.Range_hood" "None")
    (else
      (`PrimitiveComponent.CreateDynamicMaterialInstance` _buttongreen 0 "/Game/Materials/Materials_props/Range_hood_NOTEmmisive.Range_hood_NOTEmmisive" "None")
      (`PrimitiveComponent.CreateDynamicMaterialInstance` _buttonred 0 "/Game/Materials/Materials_props/Range_hood_NOTEmmisive.Range_hood_NOTEmmisive" "None"))))

(event `self.Tracker.OnComponentEndOverlap`
  (params (OverlappedComponent :type "PrimitiveComponent Object Reference") (OtherActor :type "Actor Object Reference") (OtherComp :type "PrimitiveComponent Object Reference") (OtherBodyIndex :type Integer))
  ;[1 1 1] Добавление емисии
  (goto _label_3))

(event `InputAction|Switch_Door_light`
  (params (Key :type "Key Structure"))
  (bind _spotlight (`self.SpotLight`))
  ;[1 1 1] Вкл/Выкл света
  (:`Pressed`
    (bind _asbp_first_person_character (cast `/Game/FirstPerson/Blueprints/BP_FirstPersonCharacter` (`GameplayStatics.GetPlayerCharacter` 0)))
    (if (`/Game/FirstPerson/Blueprints/BP_FirstPersonCharacter.SwitchON` _asbp_first_person_character)
      (for (_ _array_index) _spotlight
        (`SceneComponent.ToggleVisibility` (`SpotLight.SpotLightComponent` (`|GetArrayItem` _spotlight _array_index)) false))
      (else
        (`GameplayStatics.SpawnSound2D` "/Game/Sound/Door_sound/DoorNotWork.DoorNotWork" 1.0 1.0 0.0 null)))))

(fn `UserConstructionScript`)