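; BP_CardFile is an interactive card-file cabinet drawer that the player slides open and closed with E.
; Overlapping its box enables input and briefly shows a press-E hint, while leaving disables input and hides the hint.
; Pressing E plays a sound and uses a FlipFlop to play or reverse a Timeline that moves the CardFile component along its relative X axis.
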(event `self.Box.OnComponentBeginOverlap`
  (params (OverlappedComponent :type "PrimitiveComponent Object Reference") (OtherActor :type "Actor Object Reference") (OtherComp :type "PrimitiveComponent Object Reference") (OtherBodyIndex :type Integer) (bFromSweep :type Boolean) (SweepResult :type "HitResult Structure (by ref)"))
  (bind _prees_e (`self.Prees E`))
  ;[1 1 1] подсказка
  (`self.EnableInput` (`GameplayStatics.GetPlayerController` 0))
  (`SceneComponent.SetVisibility` _prees_e true false)
  (`KismetSystemLibrary.Delay` 2.0)
  (`SceneComponent.SetVisibility` _prees_e false false))

(event `self.Box.OnComponentEndOverlap`
  (params (OverlappedComponent :type "PrimitiveComponent Object Reference") (OtherActor :type "Actor Object Reference") (OtherComp :type "PrimitiveComponent Object Reference") (OtherBodyIndex :type Integer))
  ;[1 1 1] подсказка
  (`self.DisableInput` (`GameplayStatics.GetPlayerController` 0))
  (`SceneComponent.SetVisibility` (`self.Prees E`) false false))

(event `Key|E`
  (params (Key :type "Key Structure"))
  ;[1 1 1] открыть/закрыть шкафчик
  (:`Pressed`
    (cast `/Game/FirstPerson/Blueprints/BP_FirstPersonCharacter` (`GameplayStatics.GetPlayerCharacter` 0))
    (`GameplayStatics.PlaySound2D` "/Game/Sound/CardFile/CardFile.CardFile" 1.0 1.0 0.0 null null)
    (`/Engine/EditorBlueprintResources/StandardMacros.FlipFlop`
      (:`A`
        (bind (_direction _newtrack_0) (`Timeline|Timeline` :!label _label)
          (:`Update`
            (`SceneComponent.K2_SetRelativeLocation` (`self.CardFile`) (`KismetMathLibrary.MakeVector` (* _newtrack_0 -37.0)) false false))))
      (:`B`
        (goto _label :!via `Reverse`)))))

(fn `UserConstructionScript`)