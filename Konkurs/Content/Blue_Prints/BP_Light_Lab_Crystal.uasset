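; Trigger-box actor that lights up a lab's lamp fixtures, switching their panel material and showing two spot lamps.
; Box begin and end overlap both run the same chain, gated by casting player character 0, not the overlapping actor, to BP_FirstPersonCharacter.
; It creates dynamic material instances on three lamps and makes Lamp and both spot lamps visible.
; A switch-off chain with non-emissive material is unconnected, so lights never turn off here.
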(event `self.Box.OnComponentBeginOverlap`
  (params (OverlappedComponent :type "PrimitiveComponent Object Reference") (OtherActor :type "Actor Object Reference") (OtherComp :type "PrimitiveComponent Object Reference") (OtherBodyIndex :type Integer) (bFromSweep :type Boolean) (SweepResult :type "HitResult Structure (by ref)"))
  ;[1 1 1] запускает эвент смены текстур
  (cast `/Game/FirstPerson/Blueprints/BP_FirstPersonCharacter` (`GameplayStatics.GetPlayerCharacter` 0) :!label _label)
  (`PrimitiveComponent.CreateDynamicMaterialInstance` (`self.Lamp`) 0 "/Game/Materials/Materials_props_inst/Lamp_AID_HEV_Panel.Lamp_AID_HEV_Panel" "None")
  (`PrimitiveComponent.CreateDynamicMaterialInstance` (`self.Lamp1`) 0 "/Game/Materials/Materials_props_inst/Lamp_AID_HEV_Panel.Lamp_AID_HEV_Panel" "None")
  (`PrimitiveComponent.CreateDynamicMaterialInstance` (`self.Lamp2`) 0 "/Game/Materials/Materials_props_inst/Lamp_AID_HEV_Panel.Lamp_AID_HEV_Panel" "None")
  (`SceneComponent.SetVisibility` (`self.Lamp`) true false)
  (`SceneComponent.SetVisibility` (`self.SpotLamp1`) true false)
  (`SceneComponent.SetVisibility` (`self.SpotLamp2`) true false))

(event `self.Box.OnComponentEndOverlap`
  (params (OverlappedComponent :type "PrimitiveComponent Object Reference") (OtherActor :type "Actor Object Reference") (OtherComp :type "PrimitiveComponent Object Reference") (OtherBodyIndex :type Integer))
  ;[1 1 1] запускает эвент смены текстур
  (goto _label))

(fn `UserConstructionScript`)