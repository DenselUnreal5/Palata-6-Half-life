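; BP_Polka is an interactive shelf ("polka") that the player opens and closes with the Switch_Door_light input while inside its trigger box.
; The box overlap toggles input and briefly shows a PressE prompt.
; If the first-person character's SwitchON is set, a FlipFlop plays or reverses a timeline that slides the shelf, lamps and button vertically, with open/close sounds.
; Otherwise it plays a not-working sound.
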(event `self.Box.OnComponentBeginOverlap`
  (params (OverlappedComponent :type "PrimitiveComponent Object Reference") (OtherActor :type "Actor Object Reference") (OtherComp :type "PrimitiveComponent Object Reference") (OtherBodyIndex :type Integer) (bFromSweep :type Boolean) (SweepResult :type "HitResult Structure (by ref)"))
  (bind _press_e (`self.Press E`))
  (`self.EnableInput` (`GameplayStatics.GetPlayerController` 0))
  (`SceneComponent.SetVisibility` _press_e true false)
  (`KismetSystemLibrary.Delay` 2.0)
  (`SceneComponent.SetVisibility` _press_e false false))

(event `self.Box.OnComponentEndOverlap`
  (params (OverlappedComponent :type "PrimitiveComponent Object Reference") (OtherActor :type "Actor Object Reference") (OtherComp :type "PrimitiveComponent Object Reference") (OtherBodyIndex :type Integer))
  (`self.DisableInput` (`GameplayStatics.GetPlayerController` 0))
  (`SceneComponent.SetVisibility` (`self.Press E`) false false))

(event `InputAction|Switch_Door_light`
  (params (Key :type "Key Structure"))
  (:`Pressed`
    (bind _asbp_first_person_character (cast `/Game/FirstPerson/Blueprints/BP_FirstPersonCharacter` (`GameplayStatics.GetPlayerCharacter` 0)))
    (if (`/Game/FirstPerson/Blueprints/BP_FirstPersonCharacter.SwitchON` _asbp_first_person_character)
      (`/Engine/EditorBlueprintResources/StandardMacros.FlipFlop`
        (:`A`
          (`GameplayStatics.PlaySound2D` "/Game/Sound/Table_sound/Polka_Open.Polka_Open" 1.0 1.0 0.0 null null)
          (bind (_direction _newtrack_0) (`Timeline|TL_Polka` :!label _label)
            (:`Update`
              (`SceneComponent.K2_SetRelativeLocation` (`self.Polka`) (`KismetMathLibrary.MakeVector` 0.0 0.0 (* _newtrack_0 -88.0)) false false)
              (`SceneComponent.K2_SetRelativeLocation` (`self.Lamps`) (`KismetMathLibrary.MakeVector` 0.0 0.0 (+ (* _newtrack_0 -88.0) -27.0)) false false)
              (`SceneComponent.K2_SetRelativeLocation` (`self.Button`) (`KismetMathLibrary.MakeVector` 0.0 (+ _newtrack_0 58.0) (+ (* _newtrack_0 -88.0) -30.0)) false false))))
        (:`B`
          (`GameplayStatics.PlaySound2D` "/Game/Sound/Table_sound/Polka_close.Polka_close" 1.0 1.0 0.0 null null)
          (goto _label :!via `Reverse`)))
      (else
        (`GameplayStatics.PlaySound2D` "/Game/Sound/Door_sound/DoorNotWork.DoorNotWork" 1.0 1.0 0.0 null null)))))

(fn `UserConstructionScript`)